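; Ball actor whose Boll component can be launched with physics impulses and later frozen in place.
; ApplyForce pushes it away from a given origin, while ApplyForcewithDirection pushes along a supplied vector; both enable simulation and apply power as a velocity change.
; ResetForce stops simulation, moves the actor to where the Boll ended up and reattaches it to the root, repairing the detachment that physics simulation causes.
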(event EventBeginPlay)

(event Collision|EventActorBeginOverlap
  (params (OtherActor :type Actor%20Object%20Reference)))

(event EventTick
  (params (DeltaSeconds :type Float%20%28single-precision%29)))

(event EventApplyForce
  (params (forcing%20origin :type Vector :default "0, 0, 0") (power :type Float%20%28single-precision%29))
  (bind _boll (Variables|Default|Getboll))
  (Physics|SetSimulatePhysics _boll true)
  (Physics|AddImpulse _boll (* (Math|Vector|Normalize (- (Transformation|GetWorldLocation (Variables|Default|Getboll)) forcing%20origin)) power) "None" true))

(event EventApplyForcewithDirection
  (params (Direction%20vector :type Vector :default "0, 0, 0") (power :type Float%20%28single-precision%29))
  (bind _boll (Variables|Default|Getboll))
  (Physics|SetSimulatePhysics _boll true)
  (Physics|AddImpulse _boll (* Direction%20vector power) "None" true))

(event EventResetForce
  (bind _boll (Variables|Default|Getboll))
  (if (Physics|IsSimulatingPhysics _boll "None")
    (Physics|SetSimulatePhysics _boll false)
    (Transformation|SetActorLocation (Transformation|GetWorldLocation _boll) false false)
    (Transformation|AttachComponentToComponent (Variables|Default|Getboll) (Variables|Default|GetDefaultSceneRoot) "None" "KeepWorld" "KeepWorld" "KeepWorld" true)))

(fn ConstructionScript)